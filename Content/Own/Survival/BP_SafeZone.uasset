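; BP_SafeZone is a survival-mode area that hides the player from BP_Monster AI while they stand inside it.
; Each tick it flags any overlapping BP_FirstPersonCharacter as safe, then sets IsPlayerSafe and clears HasSeenPlayer on every monster's blackboard.
; When the character ends overlap, it clears the safe flag on the character and all monster blackboards.
; Monsters are found with GetAllActorsOfClass, including every frame during overlap.
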(event Collision|EventActorEndOverlap
  (params (OtherActor :type Actor%20Object%20Reference))
  (bind _asbp_first_person_character (Utilities|Casting|CastToBP_FirstPersonCharacter OtherActor))
  (Variables|/Game/Own/Player/BP_FirstPersonCharacter.BP_FirstPersonCharacter_C|SetisSafe _asbp_first_person_character false)
  (bind _outactors (Actor|GetAllActorsOfClass "/Game/Own/AI/Monster/BP_Monster.BP_Monster_C"))
  (for _array_element _outactors
    (AI|Components|Blackboard|SetValueasBool (AI|GetBlackboard _array_element) (Utilities|Name|MakeLiteralName "IsPlayerSafe") false)))

(event EventTick
  (params (DeltaSeconds :type Float%20%28single-precision%29))
  (for _array_element (Collision|GetOverlappingActors 0 :!class /Script/Engine.Actor)
    (bind _asbp_first_person_character (Utilities|Casting|CastToBP_FirstPersonCharacter _array_element))
    (Variables|/Game/Own/Player/BP_FirstPersonCharacter.BP_FirstPersonCharacter_C|SetisSafe _asbp_first_person_character true)
    (bind _outactors (Actor|GetAllActorsOfClass "/Game/Own/AI/Monster/BP_Monster.BP_Monster_C"))
    (for _array_element_2 _outactors
      (AI|Components|Blackboard|SetValueasBool (AI|GetBlackboard _array_element_2) (Utilities|Name|MakeLiteralName "IsPlayerSafe") true)
      (AI|Components|Blackboard|SetValueasBool (AI|GetBlackboard _array_element_2) (Utilities|Name|MakeLiteralName "HasSeenPlayer") false))))

(fn ConstructionScript)