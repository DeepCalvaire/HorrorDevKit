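; Survival door actor that the player opens once with Interact, optionally requiring a matching key from the character's Keys array.
; An overlap area enables input and opens a Gate only while the first-person character is nearby.
; Opening runs a timeline that lerps the mesh yaw from closed to open angle.
; Both opening and failed key attempts play a sound and report an "Important" noise event.
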(event OnComponentBeginOverlap(OpeningArea)
  (params (OverlappedComponent :type Primitive%20Component%20Object%20Reference) (OtherActor :type Actor%20Object%20Reference) (OtherComp :type Primitive%20Component%20Object%20Reference) (OtherBodyIndex :type Integer) (bFromSweep :type Boolean) (SweepResult :type Hit%20Result%20Structure%20%28by%20ref%29))
  (bind _returnvalue (Transformation|GetActorLocation))
  (bind _asbp_first_person_character (Utilities|Casting|CastToBP_FirstPersonCharacter OtherActor))
  (Input|EnableInput (Game|GetPlayerController 0))
  (Utilities|FlowControl|Gate true) ; enters at Open
)

(event OnComponentEndOverlap(OpeningArea)
  (params (OverlappedComponent :type Primitive%20Component%20Object%20Reference) (OtherActor :type Actor%20Object%20Reference) (OtherComp :type Primitive%20Component%20Object%20Reference) (OtherBodyIndex :type Integer))
  (bind _returnvalue (Transformation|GetActorLocation))
  (Utilities|Casting|CastToBP_FirstPersonCharacter OtherActor)
  (Input|DisableInput (Game|GetPlayerController 0))
  (Utilities|FlowControl|Gate true) ; enters at Close
)

(event Input|ActionEvents|InputActionInteract
  (params (Key :type Key%20Structure :default "None"))
  (bind _returnvalue (Game|GetPlayerController 0))
  (bind _returnvalue_2 (Transformation|GetActorLocation))
  (bind _returnvalue_3 (Transformation|GetActorLocation _returnvalue))
  (:Pressed
    (if (Variables|Default|GetDoesOpenWithKey)
      (bind _array_element (Utilities|Array|ForEachLoopwithBreak (Variables|/Game/Own/Player/BP_FirstPersonCharacter.BP_FirstPersonCharacter_C|GetKeys (stale OnComponentBeginOverlap(OpeningArea) _asbp_first_person_character)))
        (:LoopBody
          (if (== _array_element (Variables|Default|GetKeyIndex))
            (Variables|Default|SethasRightKey true)))
        (:Completed
          (if (Variables|Default|GethasRightKey)
            (Utilities|FlowControl|Gate true :!label _label
              (:Exit
                (if (not (Variables|Default|GetisDoorOpen))
                  (Variables|Default|SetisDoorOpen true)
                  (Audio|PlaySoundatLocation (Variables|Default|GetOpenDoorSound) _returnvalue_2 "0, 0, 0" 1.0 1.0 0.0 0 0 0 0)
                  (Class|AISenseHearing|ReportNoiseEvent _returnvalue_2 5.0 self 0.0 "Important")
                  (Utilities|FlowControl|FlipFlop
                    (:A
                      (bind _door_track (Timeline|Open/Close Play)
                        (:Update
                          (Transformation|SetRelativeRotation (Variables|Default|GetStaticMesh) (Math|Rotator|MakeRotator 0.0 0.0 (Math|Float|Lerp (Variables|Default|GetClosedAngle) (Variables|Default|GetOpenAngle) _door_track)) false false))))))))
            (else
              (Audio|PlaySoundatLocation (Variables|Default|GetCloseDoorSound) _returnvalue_3 "0, 0, 0" 1.0 1.0 0.0 0 0 0 0)
              (Class|AISenseHearing|ReportNoiseEvent _returnvalue_3 5.0 self 0.0 "Important")))))
      (else
        (goto _label)))))

(fn ConstructionScript)